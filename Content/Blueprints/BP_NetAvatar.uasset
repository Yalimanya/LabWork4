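; BP_NetAvatar is a networked avatar Blueprint whose capsule overlap with another avatar can end the game.
; On authority only, it casts the overlapped actor, not that actor's player state, to NetPlayerState and compares its team with player state index 0's.
; Unless index 0 is Red and the other is Blue, it calls EndGame on NetGameMode.
; As written, casting the same actor to both avatar and player state likely blocks that call.
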(event `self.CapsuleComponent.OnComponentBeginOverlap`
  (params (OverlappedComponent :type "PrimitiveComponent Object Reference") (OtherActor :type "Actor Object Reference") (OtherComp :type "PrimitiveComponent Object Reference") (OtherBodyIndex :type Integer) (bFromSweep :type Boolean) (SweepResult :type "HitResult Structure (by ref)"))
  (`/Engine/EditorBlueprintResources/ActorMacros.Switch Has Authority`
    (:`Authority`
      (cast `/Game/Blueprints/BP_NetAvatar` OtherActor)
      (bind _asnet_player_state (cast `NetPlayerState` OtherActor))
      (bind _asnet_player_state_2 (cast `NetPlayerState` (`GameplayStatics.GetPlayerState` 0)))
      (if (not (and (`|EnumEquality` (`.TeamID` (break `SPlayerInfo` (`NetPlayerState.PlayerInfo` _asnet_player_state_2))) "TEAM_Red") (`|EnumEquality` (`.TeamID` (break `SPlayerInfo` (`NetPlayerState.PlayerInfo` _asnet_player_state))) "TEAM_Blue")))
        (bind _asnet_game_mode (cast `NetGameMode` (`GameplayStatics.GetGameMode`)))
        (`NetGameMode.EndGame` _asnet_game_mode true)))))

(fn `UserConstructionScript`)